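; BP_SlidingDoor is a double sliding door that opens automatically when something overlaps its trigger and closes when the overlap ends.
; The Trigger component's begin and end overlap events play and reverse the OpenCloseDoor timeline, with no filter on the overlapping actor.
; The timeline's DoorTrack drives lerps that slide the left and right door meshes apart along their relative Y axis.
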(event OnComponentBeginOverlap(Trigger)
  (params (OverlappedComponent :type Primitive%20Component%20Object%20Reference) (OtherActor :type Actor%20Object%20Reference) (OtherComp :type Primitive%20Component%20Object%20Reference) (OtherBodyIndex :type Integer) (bFromSweep :type Boolean) (SweepResult :type Hit%20Result%20Structure%20%28by%20ref%29))
  (bind _door_track (Timeline|Open/CloseDoor Play)
    (:Update
      (Transformation|SetRelativeLocation (Variables|Default|GetSM_DoorLeft) (Math|Vector|MakeVector 0.0 (Math|Float|Lerp 0.0 -2.1e+02 _door_track) 0.0) false false)
      (Transformation|SetRelativeLocation (Variables|Default|GetSM_DoorRight) (Math|Vector|MakeVector 0.0 (Math|Float|Lerp 0.0 2e+02 _door_track) 0.0) false false))))

(event OnComponentEndOverlap(Trigger)
  (params (OverlappedComponent :type Primitive%20Component%20Object%20Reference) (OtherActor :type Actor%20Object%20Reference) (OtherComp :type Primitive%20Component%20Object%20Reference) (OtherBodyIndex :type Integer))
  (bind _door_track (Timeline|Open/CloseDoor Reverse)
    (:Update
      (Transformation|SetRelativeLocation (Variables|Default|GetSM_DoorLeft) (Math|Vector|MakeVector 0.0 (Math|Float|Lerp 0.0 -2.1e+02 _door_track) 0.0) false false)
      (Transformation|SetRelativeLocation (Variables|Default|GetSM_DoorRight) (Math|Vector|MakeVector 0.0 (Math|Float|Lerp 0.0 2e+02 _door_track) 0.0) false false))))

(event EventBeginPlay
  (|CallParentFunction) ; This node is disabled and will not be called.\nDrag off pins to build functionality.
)

(event Collision|EventActorBeginOverlap
  (params (OtherActor :type Actor%20Object%20Reference))
  (|CallParentFunction OtherActor) ; This node is disabled and will not be called.\nDrag off pins to build functionality.
)

(event EventTick
  (params (DeltaSeconds :type Float%20%28single-precision%29))
  (|CallParentFunction DeltaSeconds) ; This node is disabled and will not be called.\nDrag off pins to build functionality.
)

(fn ConstructionScript
  (|CallParentFunction))